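; BP_TeleportDoor is an interactable door that also teleports the first-person character when they enter its box trigger.
; Interact alternates between playing and reversing a timeline that yaws the door wing open or closed, with a Turkish open/close prompt.
; The box overlap moves the character to TpPos, converting its location from actor-local to world space while applying its rotation unconverted, regardless of door state.
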(event OnComponentBeginOverlap(Box)
  (params (OverlappedComponent :type Primitive%20Component%20Object%20Reference) (OtherActor :type Actor%20Object%20Reference) (OtherComp :type Primitive%20Component%20Object%20Reference) (OtherBodyIndex :type Integer) (bFromSweep :type Boolean) (SweepResult :type Hit%20Result%20Structure%20%28by%20ref%29))
  (bind _tppos (Variables|Default|GettpPos))
  (bind _asbp_first_person_character (Utilities|Casting|CastToBP_FirstPersonCharacter OtherActor))
  (Transformation|SetActorLocationAndRotation _asbp_first_person_character (Math|Transform|TransformLocation (Transformation|GetActorTransform) (.location _tppos)) (.rotation _tppos)))

(event EventInteract
  (Utilities|FlowControl|FlipFlop
    (:A
      (bind _opendoor (Timeline|OpenDoor Play)
        (:Update
          (Transformation|SetRelativeRotation (Variables|Default|GetDoorWing) (Math|Rotator|MakeRotator 0.0 0.0 _opendoor) false false))))
    (:B
      (Timeline|OpenDoor Reverse))))

(fn ConstructionScript)

(fn GetInteractText
  (return "Kapıyı aç/kapat [E]"))