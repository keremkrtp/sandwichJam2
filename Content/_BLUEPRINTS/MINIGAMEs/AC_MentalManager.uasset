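; Actor component on the first-person character that runs mental-test minigames, each start spending one of the MentalLives.
; StartMentalTest pauses the game, shows the cursor and opens a widget picked from MiniGameList by remaining lives, or prints a game-over message when none remain.
; HandleSuccess unpauses, closes the widget and sets the owner's CurrentMadness to a fixed value.
; HandleFail recreates the same minigame widget without spending another life.
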(event EventBeginPlay)

(event EventTick
  (params (DeltaSeconds :type Float%20%28single-precision%29)))

(fn StartMentalTest
  (Game|SetGamePaused true)
  (Variables|/Script/Engine.PlayerController|SetbShowMouseCursor (Game|GetPlayerController 0) true)
  (if (> (Variables|Default|GetMentalLives) 0)
    (Variables|Default|SetMentalLives (- (Variables|Default|GetMentalLives) 1))
    (Variables|Default|SetIsGameActive true)
    (bind _output_get (Variables|Default|SetCurrentGameClass (Utilities|Array|Get(acopy) (Variables|Default|GetMiniGameList) (- 2 (Variables|Default|GetMentalLives)))))
    (bind _returnvalue (UserInterface|CreateWidget _output_get))
    (bind _output_get_2 (Variables|Default|SetActiveWidgetRef _returnvalue))
    (UserInterface|Viewport|AddtoViewport _output_get_2 0)
    (else
      (Development|PrintString "Oyun BİTTİ"))))

(fn HandleSuccess
  (Game|SetGamePaused false)
  (Variables|/Script/Engine.PlayerController|SetbShowMouseCursor (Game|GetPlayerController 0) false)
  (Variables|Default|SetIsGameActive false)
  (Widget|RemovefromParent (Variables|Default|GetActiveWidgetRef))
  (bind _asbp_first_person_character (Utilities|Casting|CastToBP_FirstPersonCharacter (Components|GetOwner)))
  (Variables|/Game/FirstPerson/Blueprints/BP_FirstPersonCharacter.BP_FirstPersonCharacter_C|SetCurrentMadness _asbp_first_person_character 5e+01))

(fn HandleFail
  (CallFunction|RestartCurrentGame))

(fn RestartCurrentGame
  (Utilities|IsValid (Variables|Default|GetActiveWidgetRef)
    (:Is%20Valid
      (Widget|RemovefromParent (Variables|Default|GetActiveWidgetRef))
      (bind _returnvalue (UserInterface|CreateWidget (Variables|Default|GetCurrentGameClass)))
      (bind _output_get (Variables|Default|SetActiveWidgetRef _returnvalue))
      (UserInterface|Viewport|AddtoViewport _output_get 0))))